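; Ronces_BP is a bramble hazard actor that hurts the player on contact.
; On BeginPlay it casts and caches the player's ThirdPersonCharacter.
; When that character begins overlapping its Box component, it directly subtracts a fixed amount from the character's Life variable and prints the new value, without using the damage system.
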(event `self.ReceiveBeginPlay`
  (bind _asthird_person_character (cast `/Game/Matthieu_Dubuisson/ThirdPersonCharacter` (`GameplayStatics.GetPlayerCharacter` 0)))
  (set `self.Third Person Character` _asthird_person_character))

(event `self.Box.OnComponentBeginOverlap`
  (params (OverlappedComponent :type "PrimitiveComponent Object Reference") (OtherActor :type "Actor Object Reference") (OtherComp :type "PrimitiveComponent Object Reference") (OtherBodyIndex :type Integer) (bFromSweep :type Boolean) (SweepResult :type "HitResult Structure (by ref)"))
  (bind _third_person_character (`self.Third Person Character`))
  (if (== _third_person_character OtherActor)
    (bind _output_get (set `/Game/Matthieu_Dubuisson/ThirdPersonCharacter.Life` (- (`/Game/Matthieu_Dubuisson/ThirdPersonCharacter.Life` _third_person_character) 5.0) _third_person_character))
    (`KismetSystemLibrary.PrintString` (`KismetStringLibrary.Conv_DoubleToString` _output_get))))

(fn `UserConstructionScript`)