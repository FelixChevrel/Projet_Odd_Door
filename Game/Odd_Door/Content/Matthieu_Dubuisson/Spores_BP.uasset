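; Spores hazard actor that poisons the player character while it stands inside the Box trigger.
; It caches the player's ThirdPersonCharacter on BeginPlay and reacts only to that character's overlaps.
; Entering starts a looping half-second timer that decrements the character's Life and prints it while an Activate flag is set.
; Leaving only clears the flag, so the timer keeps running without applying damage.
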(event `self.ReceiveBeginPlay`
  (bind _asthird_person_character (cast `/Game/Matthieu_Dubuisson/ThirdPersonCharacter` (`GameplayStatics.GetPlayerCharacter` 0)))
  (set `self.ThirdPersonCharacter` _asthird_person_character))

(event `self.Box.OnComponentBeginOverlap`
  (params (OverlappedComponent :type "PrimitiveComponent Object Reference") (OtherActor :type "Actor Object Reference") (OtherComp :type "PrimitiveComponent Object Reference") (OtherBodyIndex :type Integer) (bFromSweep :type Boolean) (SweepResult :type "HitResult Structure (by ref)"))
  (if (== (`self.ThirdPersonCharacter`) OtherActor)
    (set `self.Activate` true)
    (`KismetSystemLibrary.K2_SetTimerDelegate` (delegate `Poison`) 0.5 true)))

(event `Poison`
  (bind _thirdpersoncharacter (`self.ThirdPersonCharacter`))
  (bind _life (`/Game/Matthieu_Dubuisson/ThirdPersonCharacter.Life` _thirdpersoncharacter))
  (if (`self.Activate`)
    (set `/Game/Matthieu_Dubuisson/ThirdPersonCharacter.Life` (- _life 1.0) _thirdpersoncharacter)
    (`KismetSystemLibrary.PrintString` (`KismetStringLibrary.Conv_DoubleToString` _life))))

(event `self.Box.OnComponentEndOverlap`
  (params (OverlappedComponent :type "PrimitiveComponent Object Reference") (OtherActor :type "Actor Object Reference") (OtherComp :type "PrimitiveComponent Object Reference") (OtherBodyIndex :type Integer))
  (if (== (`self.ThirdPersonCharacter`) OtherActor)
    (set `self.Activate` false)))

(fn `UserConstructionScript`)