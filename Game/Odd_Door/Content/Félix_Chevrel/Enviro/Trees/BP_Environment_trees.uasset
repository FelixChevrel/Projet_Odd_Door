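; Environment tree actor that picks one of four tree meshes from its Type setting, with randomized wood and leaf materials.
; The construction script sets the mesh, then draws wood and leaf materials independently from four-entry random picks in ColorLibrary, re-rolled on each reconstruction.
; Material slot indices are swapped for Trees_1, whose wood and leaf slots are reversed relative to the other meshes.
; The event graph has no gameplay logic.
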(fn `UserConstructionScript`
  (bind _trees (`self.Trees`))
  (bind (_colorlibrary_woodmat _colorlibrary_leafmat) (break `/Game/Félix_Chevrel/Material/Plants/STRUCT_Wood_Random_material` (`self.ColorLibrary`)))
  (bind _returnvalue (select `int` (`self.Type`) :`0` "/Game/Félix_Chevrel/Enviro/Trees/Trees_1.Trees_1" :`1` "/Game/Félix_Chevrel/Enviro/Trees/Trees_2.Trees_2" :`2` "/Game/Félix_Chevrel/Enviro/Trees/Trees_3.Trees_3" :`3` "/Game/Félix_Chevrel/Enviro/Trees/Trees_4.Trees_4" :!type "StaticMesh Object Reference"))
  (bind _returnvalue_2 (== _returnvalue "/Game/Félix_Chevrel/Enviro/Trees/Trees_1.Trees_1"))
  (`StaticMeshComponent.SetStaticMesh` _trees _returnvalue)
  (`PrimitiveComponent.SetMaterial` _trees (`KismetMathLibrary.SelectInt` 1 0 _returnvalue_2) (`|GetArrayItem` _colorlibrary_woodmat (`KismetMathLibrary.RandomInteger` 4)))
  (`PrimitiveComponent.SetMaterial` _trees (`KismetMathLibrary.SelectInt` 0 1 _returnvalue_2) (`|GetArrayItem` _colorlibrary_leafmat (`KismetMathLibrary.RandomInteger` 4))))