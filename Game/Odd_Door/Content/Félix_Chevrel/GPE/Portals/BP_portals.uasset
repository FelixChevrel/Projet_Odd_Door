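; BP_portals is a linked portal actor that teleports the player's third-person character to a paired portal.
; When the player hits it and OtherPortal is valid, it plays a 2D sound and moves the player to that portal's exit transform.
; It then sets the camera boom rotation to the mesh's relative rotation.
; The construction script applies the configurable plane transform, exit point and material on both planes.
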(event `self.ReceiveBeginPlay`
  (bind _asthird_person_character (cast `/Game/Matthieu_Dubuisson/ThirdPersonCharacter` (`GameplayStatics.GetPlayerPawn` 0)))
  (set `self.PlayerRef` _asthird_person_character))

(event `self.ReceiveHit`
  (params (MyComp :type "PrimitiveComponent Object Reference") (Other :type "Actor Object Reference") (OtherComp :type "PrimitiveComponent Object Reference") (bSelfMoved :type Boolean) (HitLocation :type "Vector Structure") (HitNormal :type "Vector Structure") (NormalImpulse :type "Vector Structure") (Hit :type "HitResult Structure (by ref)"))
  (bind _playerref (`self.PlayerRef`))
  (if (and (`KismetSystemLibrary.IsValid` (`self.OtherPortal`)) (== _playerref Other))
    (`GameplayStatics.PlaySound2D` "/Engine/VREditor/Sounds/UI/Teleport_Committed.Teleport_Committed" 1.0 1.0 0.0 null null)
    (`self.K2_SetActorTransform` _playerref (`SceneComponent.K2_GetComponentToWorld` (`/Game/Félix_Chevrel/GPE/Portals/BP_portals.ExitRef` (`self.OtherPortal`))) false false)
    (`SceneComponent.K2_SetRelativeRotation` (`/Game/Matthieu_Dubuisson/ThirdPersonCharacter.CameraBoom` _playerref) (`SceneComponent.RelativeRotation` (`Character.Mesh` _playerref)) false false)))

(fn `UserConstructionScript`
  (bind _exitref (`self.ExitRef`))
  (bind _material (`self.Material`))
  ;[1 1 1] Set portal & exit location
  (`SceneComponent.K2_SetRelativeTransform` (`self.Plane`) (`self.Portal_transform`) false false)
  (`SceneComponent.K2_SetRelativeLocation` _exitref (`self.exit_location`) false false)
  (`SceneComponent.K2_SetRelativeRotation` _exitref (`self.exit_rotation`) false false)
  ;[1 1 1] Set Material
  (`PrimitiveComponent.SetMaterial` (`self.Plane`) 0 _material)
  (`PrimitiveComponent.SetMaterial` (`self.Plane1`) 0 _material))