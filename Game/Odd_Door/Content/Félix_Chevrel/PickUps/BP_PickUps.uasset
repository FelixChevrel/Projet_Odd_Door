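; Pickup actor that the player collects by walking into its box, as long as they are not already holding something.
; On overlap it copies its mesh onto the ThirdPersonCharacter's CaughtObject, sets the holding flag and destroys itself.
; The construction script applies the Mesh variable to both the visible Cube and a CubeHighlight duplicate, whose material slots all get an outline material.
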(event `self.ReceiveBeginPlay`
  (bind _asthird_person_character (cast `/Game/Matthieu_Dubuisson/ThirdPersonCharacter` (`GameplayStatics.GetPlayerPawn` 0)))
  (set `self.PlayerRef` _asthird_person_character))

(event `self.Box.OnComponentBeginOverlap`
  (params (OverlappedComponent :type "PrimitiveComponent Object Reference") (OtherActor :type "Actor Object Reference") (OtherComp :type "PrimitiveComponent Object Reference") (OtherBodyIndex :type Integer) (bFromSweep :type Boolean) (SweepResult :type "HitResult Structure (by ref)"))
  (bind _playerref (`self.PlayerRef`))
  (if (and (== OtherActor _playerref) (not (`/Game/Matthieu_Dubuisson/ThirdPersonCharacter.Is_holding_Something` _playerref)))
    (`StaticMeshComponent.SetStaticMesh` (`/Game/Matthieu_Dubuisson/ThirdPersonCharacter.Caught_Object` _playerref) (`StaticMeshComponent.StaticMesh` (`self.Cube`)))
    (set `/Game/Matthieu_Dubuisson/ThirdPersonCharacter.Is_holding_Something` true _playerref)
    (`self.K2_DestroyActor`)))

(fn `UserConstructionScript`
  (bind _mesh (`self.Mesh`))
  (bind _cube_highlight (`self.Cube_highlight`))
  (`StaticMeshComponent.SetStaticMesh` (`self.Cube`) _mesh)
  (`StaticMeshComponent.SetStaticMesh` _cube_highlight _mesh)
  (for (_ _array_index) (`MeshComponent.GetMaterials` _cube_highlight)
    (`PrimitiveComponent.SetMaterial` (`self.Cube_highlight`) _array_index "/Game/Félix_Chevrel/Material/MAT_GPE_outline.M_GPE_outline")))