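; Item drop-off point where the player deposits the object they are carrying.
; On BeginPlay it caches the ThirdPersonCharacter pawn, then waits for that player to overlap its Box while holding something.
; The overlap moves the held static mesh onto Decor, clears the player's holding state, destroys the Cube component and sets Filled.
; Filled is not checked here, so a later deposit replaces the Decor mesh.
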(event `self.ReceiveBeginPlay`
  (bind _asthird_person_character (cast `/Game/Matthieu_Dubuisson/ThirdPersonCharacter` (`GameplayStatics.GetPlayerPawn` 0)))
  (set `self.PlayerRef` _asthird_person_character))

(event `self.Box.OnComponentBeginOverlap`
  (params (OverlappedComponent :type "PrimitiveComponent Object Reference") (OtherActor :type "Actor Object Reference") (OtherComp :type "PrimitiveComponent Object Reference") (OtherBodyIndex :type Integer) (bFromSweep :type Boolean) (SweepResult :type "HitResult Structure (by ref)"))
  (bind _playerref (`self.PlayerRef`))
  (bind _playerref_2 (`self.PlayerRef`))
  (if (and (== OtherActor _playerref) (`/Game/Matthieu_Dubuisson/ThirdPersonCharacter.Is_holding_Something` _playerref))
    (`StaticMeshComponent.SetStaticMesh` (`self.Decor`) (`StaticMeshComponent.StaticMesh` (`/Game/Matthieu_Dubuisson/ThirdPersonCharacter.Caught_Object` _playerref)))
    (`StaticMeshComponent.SetStaticMesh` (`/Game/Matthieu_Dubuisson/ThirdPersonCharacter.Caught_Object` _playerref_2) null)
    (set `/Game/Matthieu_Dubuisson/ThirdPersonCharacter.Is_holding_Something` false _playerref_2)
    (`ActorComponent.K2_DestroyComponent` (`self.Cube`))
    (set `self.Filled` true)))

(fn `UserConstructionScript`)