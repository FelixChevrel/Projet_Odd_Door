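; BP_Decoration_manager tracks whether all decoration spots are filled, as the win condition of a decoration objective.
; Each call to its Check event increments an object counter, then scans the Spots array and clears Validated if any spot is not Filled.
; The result is only printed as a victory or "not yet" debug string, and the counter does not affect it.
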(event `Check`
  (set `self.Validated` true)
  (set `self.NbObjects` (+ (`self.NbObjects`) 1))
  (for _array_element (`self.Spots`)
    (if (not (`/Game/Félix_Chevrel/PickUps/BP_Dépots_Items.Filled` _array_element))
      (set `self.Validated` false)))
  (if (`self.Validated`)
    (`KismetSystemLibrary.PrintString` "\"victory\"")
    (else
      (`KismetSystemLibrary.PrintString` "not yet"))))

(fn `UserConstructionScript`)